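; Health component that tracks hit points for its owner and exposes get, set, damage, heal and restore functions.
; On BeginPlay it binds to the owner's OnTakeAnyDamage, which feeds incoming damage into DamageHP.
; When IsCharacter is set and no health remains, it sets the mesh's physics blend weight to full and unpossesses the AI controller.
; HealHP checks MaxHealth before adding but does not clamp the result.
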(event Custom|TakeDamage
  (params (DamagedActor :type Actor%20Object%20Reference) (Damage :type Float%20%28single-precision%29) (DamageType :type Damage%20Type%20Object%20Reference) (InstigatedBy :type Controller%20Object%20Reference) (DamageCauser :type Actor%20Object%20Reference))
  (bind _returnvalue (Components|GetOwner))
  (bind _has_hp (Health|DamageHP Damage))
  (if (Variables|Default|GetIsCharacter)
    (if (not _has_hp)
      (bind _ascharacter (Utilities|Casting|CastToCharacter _returnvalue))
      (Class|SkeletalMeshComponent|SetPhysicsBlendWeight (Variables|/Script/Engine.Character|GetMesh _ascharacter) 1.0)
      (Pawn|UnPossess (AI|GetAIController _returnvalue)))))

(event EventBeginPlay
  (EventDispatchers|BindEventtoOnTakeAnyDamage (Components|GetOwner) (delegate Custom|TakeDamage)))

(fn GetHP
  (bind _health (Variables|Health|GetHealth))
  (return _health (> _health 0.0)))

(fn HealHP
  (params (Amount :type Float%20%28single-precision%29))
  (if (< (Variables|Health|GetHealth) (Variables|Health|GetMaxHealth))
    (Variables|Health|SetHealth (+ Amount (Variables|Health|GetHealth)))
    (return (< (Variables|Health|GetHealth) (Variables|Health|GetMaxHealth)))))

(fn RestoreHP
  (Variables|Health|SetHealth (Variables|Health|GetMaxHealth)))

(fn DamageHP
  (params (Damage :type Float%20%28single-precision%29))
  (if (> (Variables|Health|GetHealth) 0.0)
    (Variables|Health|SetHealth (- (Variables|Health|GetHealth) Damage))
    (return (> (Variables|Health|GetHealth) 0.0))))

(fn SetHP
  (params (Health :type Float%20%28single-precision%29))
  (Variables|Health|SetHealth Health))