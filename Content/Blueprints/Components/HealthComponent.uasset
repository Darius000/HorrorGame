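; Actor component that tracks the owning actor's health, with functions to get, set, refill, add or subtract it and check whether it is alive.
; On BeginPlay it binds to the owner's OnTakeAnyDamage and fills Health to MaxHealth.
; Damage routes through HealHealth as a negative amount, so its below-max check ignores damage at full health.
; TakeHealth subtracts only above zero but is unused here, and neither function clamps the result.
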(event Custom|TakeDamage
  (params (DamagedActor :type Actor%20Object%20Reference) (Damage :type Float%20%28single-precision%29) (DamageType :type Damage%20Type%20Object%20Reference) (InstigatedBy :type Controller%20Object%20Reference) (DamageCauser :type Actor%20Object%20Reference))
  (Health|HealHealth (* Damage -1.0)))

(event EventBeginPlay
  (EventDispatchers|BindEventtoOnTakeAnyDamage (Components|GetOwner) (delegate Custom|TakeDamage))
  (Health|SetFullHealth))

(fn GetHealth
  (return (Variables|Health|GetHealth)))

(fn HealHealth
  (params (Amount :type Float%20%28single-precision%29))
  (if (< (Variables|Health|GetHealth) (Variables|Health|GetMaxHealth))
    (Variables|Health|SetHealth (+ Amount (Variables|Health|GetHealth)))))

(fn SetFullHealth
  (Variables|Health|SetHealth (Variables|Health|GetMaxHealth)))

(fn GetIsAlive
  (return (> (Variables|Health|GetHealth) 0.0)))

(fn SetHealth
  (params (Health :type Float%20%28single-precision%29))
  (Variables|Health|SetHealth Health))

(fn TakeHealth
  (params (Amount :type Float%20%28single-precision%29))
  (if (> (Variables|Health|GetHealth) 0.0)
    (Variables|Health|SetHealth (- (Variables|Health|GetHealth) Amount))))