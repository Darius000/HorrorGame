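; Door actor that players open, close and unlock with a matching inventory key, with overlap-driven opening for the Automatic door type.
; Construction loads meshes, sounds, key and initial state from the fixed StorageRoom row of the door data table.
; A timeline swings the door yaw, signed by the pawn's world forward X, and reverses to close.
; Interaction and overlap logic both run only while the AutoMatic flag is false.
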(event OnComponentBeginOverlap(Box)
  (params (OverlappedComponent :type Primitive%20Component%20Object%20Reference) (OtherActor :type Actor%20Object%20Reference) (OtherComp :type Primitive%20Component%20Object%20Reference) (OtherBodyIndex :type Integer) (bFromSweep :type Boolean) (SweepResult :type Hit%20Result%20Structure%20%28by%20ref%29))
  ;[0.3604 1 0.9302] For Automatic Door
  (if (not (Variables|State|GetAutoMatic))
    (bind _aspawn (Utilities|Casting|CastToPawn OtherActor))
    (switch Utilities|FlowControl|Switch|SwitchonENUM_Door (.Door (Utilities|Struct|BreakSTRUCT_Door (Variables|DoorProperties|GetDoorProperties)))
      (:NewEnumerator1
        (CallFunction|OpenDoor _aspawn)))))

(event OnComponentEndOverlap(Box)
  (params (OverlappedComponent :type Primitive%20Component%20Object%20Reference) (OtherActor :type Actor%20Object%20Reference) (OtherComp :type Primitive%20Component%20Object%20Reference) (OtherBodyIndex :type Integer))
  ;[0.3604 1 0.9302] For Automatic Door
  (if (not (Variables|State|GetAutoMatic))
    (Utilities|Casting|CastToPawn OtherActor)
    (switch Utilities|FlowControl|Switch|SwitchonENUM_Door (.Door (Utilities|Struct|BreakSTRUCT_Door (Variables|DoorProperties|GetDoorProperties)))
      (:NewEnumerator1
        (CallFunction|CloseDoor)))))

(event Custom|OpenDoor
  (params (Pawn :type Pawn%20Object%20Reference))
  ;[1 0.6695 0] Opens Door if not opening
  (if (not (Variables|State|GetIsOpening?))
    (Variables|Pawn|SetDirection (Pawn|GetPawnForwardDirection Pawn))
    (Variables|State|SetIsOpened true)
    (Variables|State|SetIsOpening? true)
    (Sound|PlaySoundArray)
    ;[1 0.02604 0.02604] Door Animation
    (bind _alpha (Timeline|DoorAnim Play)
      (:Update
        (Transformation|SetRelativeRotation (Variables|Default|GetDoor) (Math|Rotator|MakeRotator 0.0 0.0 (* _alpha (Variables|Pawn|GetDirection))) false false))
      (:Finished
        (if (Variables|State|GetIsOpening?)
          (Variables|State|SetIsOpening? false))))))

(event Custom|CloseDoor
  ;[1 0.6672 0] Is Door not Opening if so play sound and close
  (if (not (Variables|State|GetIsOpening?))
    (Variables|State|SetIsOpened false)
    (Sound|PlaySoundArray 1)
    ;[1 0.02604 0.02604] Door Animation
    (bind _alpha (Timeline|DoorAnim Reverse)
      (:Update
        (Transformation|SetRelativeRotation (Variables|Default|GetDoor) (Math|Rotator|MakeRotator 0.0 0.0 (* _alpha (Variables|Pawn|GetDirection))) false false))
      (:Finished
        (if (Variables|State|GetIsOpening?)
          (Variables|State|SetIsOpening? false))))))

(event EventInteract
  (params (Character :type Character%20Object%20Reference))
  (bind _doorproperties (Variables|DoorProperties|GetDoorProperties))
  (bind _doorkey (Utilities|Struct|BreakSTRUCT_Door _doorproperties))
  ;[0.2964 0.7018 1] Door Interaction
  (Variables|Pawn|SetCharacter Character)
  (if (not (Variables|State|GetAutoMatic))
    (if (Variables|State|GetIsLocked) ; Is Door Unlocked
      ;[1 0.7041 0.2686] Check If Door Can Unlcok
      (bind _output (Default|GetItems (Variables|/Game/ThirdPersonBP/Blueprints/ThirdPersonCharacter.ThirdPersonCharacter_C|GetInventoryComponent (.AsThird%20Person%20Character (Utilities|Casting|CastToThirdPersonCharacter (Variables|Pawn|GetCharacter)))) _doorkey))
      (if (Utilities|Enum|Equal(Enum) _output _doorkey)
        (Sound|PlaySoundArray 3)
        (Variables|State|SetIsLocked false)
        (else
          (Sound|PlaySoundArray 4)))
      (else
        ;[0.7012 0.5831 1] Opens And Close Door
        (if (not (Variables|State|GetIsOpened))
          (CallFunction|OpenDoor (Variables|Pawn|GetCharacter))
          (else
            (CallFunction|CloseDoor)))))))

(fn ConstructionScript
  (bind _returnvalue (Utilities|GetDataTableRow "/Game/Blueprints/Doors/DATATABLE_Door.DATATABLE_Door" (Variables|Default|GetStorageRoom))
    (:then
      (Variables|DoorProperties|SetDoorProperties _returnvalue)
      (Utilities|FlowControl|Sequence
        (:then_0
          ;[0.2686 0.8699 1] Get Door Current Location
          (Variables|Pawn|SetDoorLocation (Transformation|GetActorLocation)))
        (:then_1
          ;[1 0.2527 0] Set Door Meshes
          (Components|StaticMesh|SetStaticMesh (Variables|Default|GetFrame) (Utilities|Array|Get(acopy) (.doormeshes (Variables|DoorProperties|GetDoorProperties))))
          (Components|StaticMesh|SetStaticMesh (Variables|Default|GetDoor) (Utilities|Array|Get(acopy) (.doormeshes (Variables|DoorProperties|GetDoorProperties)) 1)))
        (:then_2
          ;[1 0.4095 0.3397] Set Door isLocked and isOpened (IsOpened only set if isLocked = false)
          (Variables|State|SetAutoMatic (.automatic (Variables|DoorProperties|GetDoorProperties)))
          (Variables|State|SetIsLocked (.locked (Variables|DoorProperties|GetDoorProperties)))
          (bind _output_get (Variables|State|SetIsOpened (.isopened (Variables|DoorProperties|GetDoorProperties))))
          (if _output_get
            (LocalVariables|SetRotation 9e+01)
            (else
              (LocalVariables|SetRotation 0.0)))
          (Transformation|SetRelativeRotation (Variables|Default|GetDoor) (Math|Rotator|MakeRotator 0.0 0.0 (LocalVariables|GetRotation)) false false))))))

(fn CompareNames
  (params (KeyName :type String) (DoorName :type String))
  (return (Utilities|Enum|Equal(Enum) KeyName DoorName)))

(fn PlaySoundArray
  (params (Index :type Integer))
  (bind _doorproperties (Variables|DoorProperties|GetDoorProperties))
  (bind _output (Utilities|Array|Get(acopy) (.doorsounds _doorproperties) Index))
  (if (!= _output 0)
    (Audio|PlaySoundatLocation _output (Variables|Pawn|GetDoorLocation))
    (return (Variables|/Script/Engine.SoundBase|GetDuration _output))))

(fn GetPawnForwardDirection
  (params (Actor :type Actor%20Object%20Reference))
  (if (>= (.x (Transformation|GetActorForwardVector Actor)) 0.0)
    (LocalVariables|SetXDirection 1.0)
    (return (LocalVariables|GetXDirection))
    (else
      (LocalVariables|SetXDirection -1.0)
      (return (LocalVariables|GetXDirection)))))