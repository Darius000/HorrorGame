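; SaveManager actor that keeps a per-level MasterSave of interacted objects, using the current level name as the slot.
; On BeginPlay it loads an existing save and sends InteractedWithMessage to each recorded object, or creates a new save object.
; AddInteractedObject appends to the saved list, while writing to disk happens only in Save.
; EndPlay deletes the level's slot on a level transition, so progress does not carry across transitions.
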(event EventBeginPlay
  (bind _returnvalue (Game|GetCurrentLevelName true))
  (bind _returnvalue_2 (SaveGame|DoesSaveGameExist _returnvalue))
  (if _returnvalue_2
    (CallFunction|Load)
    (else
      (bind _returnvalue_3 (SaveGame|CreateSaveGameObject "/Game/Blueprints/SaveSystem/MasterSave.MasterSave_C"))
      (Variables|Default|SetCurrentSaveGame _returnvalue_3))))

(event EventEndPlay
  (params (EndPlayReason :type EEndPlayReason%20Enum :default "Destroyed"))
  (if (Utilities|Enum|Equal(Enum) EndPlayReason "LevelTransition")
    (bind _returnvalue (Game|GetCurrentLevelName true))
    (SaveGame|DeleteGameinSlot _returnvalue)))

(fn ConstructionScript)

(fn Save
  (bind _currentsavegame (Variables|Default|GetCurrentSaveGame))
  (bind _returnvalue (Game|GetCurrentLevelName true))
  (bind _output_get (Variables|/Game/Blueprints/SaveSystem/MasterSave.MasterSave_C|SetLevelSaved _currentsavegame _returnvalue))
  (bind _returnvalue_2 (SaveGame|SaveGametoSlot _currentsavegame _output_get))
  (return _returnvalue_2))

(fn Load
  (bind _returnvalue (Game|GetCurrentLevelName true))
  (bind _returnvalue_2 (SaveGame|LoadGamefromSlot _returnvalue))
  (bind _asmaster_save (Utilities|Casting|CastToMasterSave _returnvalue_2))
  (bind _output_get (Variables|Default|SetCurrentSaveGame _asmaster_save))
  (if (!= _output_get 0)
    (for _array_element (Variables|/Game/Blueprints/SaveSystem/MasterSave.MasterSave_C|GetSavedObjects _output_get)
      (Class|SaveInterface|InteractedWith?(Message) (.Object (Utilities|Struct|BreakObjectIdentifier _array_element)) true))
    (return)))

(fn AddInteractedObject
  (params (ObjectID :type Object%20Identifier%20Structure))
  (Utilities|Array|Add (Variables|/Game/Blueprints/SaveSystem/MasterSave.MasterSave_C|GetSavedObjects (Variables|Default|GetCurrentSaveGame)) ObjectID))