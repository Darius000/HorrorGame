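; Battery pickup actor that recharges the player's flashlight when grabbed into the inventory.
; Grab calls the parent Grab logic, then requires the grabber to be a ThirdPersonCharacter.
; When AddToInventory is set, it calls AddBatery on the character's child-actor Flashlight if that is the held class, then destroys itself regardless.
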(event EventBeginPlay)

(event Collision|EventActorBeginOverlap
  (params (OtherActor :type Actor%20Object%20Reference)))

(event EventTick
  (params (DeltaSeconds :type Float%20%28single-precision%29)))

(event EventGrab
  (params (Chracter :type Character%20Object%20Reference) (AddToInventory :type Boolean))
  (|CallParentFunction Chracter AddToInventory)
  (bind _asthird_person_character (Utilities|Casting|CastToThirdPersonCharacter Chracter))
  (if AddToInventory
    (Utilities|FlowControl|Sequence
      (:then_0
        (if (== (Variables|/Script/Engine.ChildActorComponent|GetChildActorClass (Variables|/Game/ThirdPersonBP/Blueprints/ThirdPersonCharacter.ThirdPersonCharacter_C|GetObject _asthird_person_character)) "/Game/Blueprints/Lights/Flashlight/Flashlight.Flashlight_C")
          (bind _asflashlight (Utilities|Casting|CastToFlashlight (Variables|/Script/Engine.ChildActorComponent|GetChildActor (Variables|/Game/ThirdPersonBP/Blueprints/ThirdPersonCharacter.ThirdPersonCharacter_C|GetObject _asthird_person_character))))
          (Default|AddBatery _asflashlight)))
      (:then_1
        (Actor|DestroyActor)))))

(fn ConstructionScript)