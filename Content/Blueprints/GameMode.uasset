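; Game mode that starts loading saved message data for the current level through a SaveManager actor.
; On BeginPlay it finds the first SaveManager in the world, then calls LoadMessage using the level name as slot and the first player's controller ID as user.
; EndPlay checks for quit or end of editor play but does nothing, and a save slot deletion node is left disconnected.
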(event EventBeginPlay
  (Utilities|FlowControl|Sequence
    (:then_0
      (bind _outactors (Actor|GetAllActorsOfClass "/Game/Blueprints/Saving/SaveManager.SaveManager_C"))
      (Variables|Default|SetSaveManager (Utilities|Array|Get(acopy) _outactors)))
    (:then_1
      (bind _returnvalue (Class|GameplayStatics|GetPlayerControllerID (Game|GetPlayerController 0)))
      (Variables|Default|SetID _returnvalue)
      (bind _returnvalue_2 (Game|GetCurrentLevelName true))
      (Variables|Default|SetLevelName _returnvalue_2)
      (Class|SaveLoad|Load(Message) (Variables|Default|GetSaveManager) (Variables|Default|GetLevelName) (Variables|Default|GetID)))))

(event EventEndPlay
  (params (EndPlayReason :type EEndPlayReason%20Enum :default "Destroyed"))
  (if (or (Utilities|Enum|Equal(Enum) EndPlayReason "Quit") (Utilities|Enum|Equal(Enum) EndPlayReason "EndPlayInEditor"))
    _))

(fn ConstructionScript)