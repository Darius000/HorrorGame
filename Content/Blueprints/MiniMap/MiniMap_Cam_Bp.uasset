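; Minimap camera actor that follows the player with a SceneCaptureComponent2D.
; On BeginPlay it adds the MiniMap_UI widget to the viewport, then after a short delay attaches a rotated, scaled-down Paper sprite component above the player character.
; Each tick it copies the player pawn's world X and Y into the capture's relative location, keeping its height and rotation fixed.
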(event EventBeginPlay
  (bind _returnvalue (UserInterface|CreateWidget "/Game/Blueprints/MiniMap/MiniMap_UI.MiniMap_UI_C"))
  (UserInterface|Viewport|AddtoViewport _returnvalue 0)
  (Utilities|FlowControl|Delay 0.2)
  (AddComponent|AddPaperSpriteComponent (Game|GetPlayerCharacter 0) false (Math|Transform|MakeTransform "0, 0,270.000000" "0, 0,90.000000" "0.500000,0.500000,0.500000")))

(event EventTick
  (params (DeltaSeconds :type Float%20%28single-precision%29))
  (bind _returnvalue (Game|Player|GetPlayerPawn 0))
  (bind _scenecapturecomponent2d (Variables|Default|GetSceneCaptureComponent2D))
  (bind _returnvalue_2 (Transformation|GetActorLocation _returnvalue))
  (bind _relativerotation (Variables|/Script/Engine.SceneComponent|GetRelativeRotation _scenecapturecomponent2d))
  (bind (_x _y) (Math|Vector|BreakVector _returnvalue_2))
  (bind (_roll _pitch) (Math|Rotator|BreakRotator _relativerotation))
  (Transformation|SetRelativeLocationAndRotation (Variables|Default|GetSceneCaptureComponent2D) (Math|Vector|MakeVector _x _y (.Z (Math|Vector|BreakVector (Variables|/Script/Engine.SceneComponent|GetRelativeLocation _scenecapturecomponent2d)))) (Math|Rotator|MakeRotator _roll _pitch (.Yaw (Math|Rotator|BreakRotator _relativerotation))) false false))

(fn ConstructionScript)