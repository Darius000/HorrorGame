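; Save manager that, when a ThirdPersonCharacter interacts, loads or creates a GameSave in a slot named after the current level.
; It then sends GetSavableValuesMessage to every actor implementing SaveAble_Bp.
; For existing saves this runs through a delayed, iterator-based batching loop whose continuation return is unwired.
; SaveAllObjects writes one SavableObject entry into the save array and saves the slot, only when an existing save was loaded.
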(event Custom|LoadSavableObjectsInto%20Array
  (params (Current%20Iterator :type Integer))
  ;[1 1 1] Loop for Loading Savable Objects from scene into array
  (bind (_next_iterator _should_run_again) (CallFunction|LoadSaveableObjectsIntoArray Current%20Iterator))
  (Utilities|FlowControl|Delay 0.0)
  (if _should_run_again
    (CallFunction|LoadSaveableObjectsIntoArray _next_iterator)))

(event Custom|SaveAllObjects
  (Variables|Default|SetUpdatedSaveObject false)
  (if (Variables|Default|GetLoadedFromSaveGame?)
    (Utilities|Array|SetArrayElem (Variables|/Game/Blueprints/Saving/GameSave.GameSave_C|GetSaveableObjects (Variables|SaveActor|GetGameSave)) (Variables|Default|GetLoaded%20Savable%20object%20Index) (Variables|Default|GetSavableObject))
    (SaveGame|SaveGametoSlot (Variables|SaveActor|GetGameSave) (Variables|SaveName|GetLevelName))))

(event EventInteract
  (params (Character :type Character%20Object%20Reference))
  (Utilities|Casting|CastToThirdPersonCharacter Character)
  (bind _returnvalue (Game|GetCurrentLevelName true))
  (Variables|SaveName|SetLevelName _returnvalue)
  (bind (_asgame_save _loadedfromsavegame_) (CallFunction|CreateorLoadSaveGame (Variables|SaveName|GetLevelName) 0 "/Game/Blueprints/Saving/GameSave.GameSave_C"))
  (if _loadedfromsavegame_
    (bind _outactors (Actor|GetAllActorswithInterface "/Game/Blueprints/Saving/SaveAble_Bp.SaveAble_Bp_C"))
    (Variables|Default|SetCached%20SavableObjects _outactors)
    (CallFunction|LoadSavableObjectsIntoArray)
    (else
      (bind _outactors_2 (Actor|GetAllActorswithInterface "/Game/Blueprints/Saving/SaveAble_Bp.SaveAble_Bp_C"))
      (for _array_element _outactors_2
        (Class|SaveAbleBp|GetSavableValues(Message) _array_element)))))

(fn ConstructionScript)

(fn CreateorLoadSaveGame
  (params (SlotName :type String) (UserIndex :type Integer) (SaveGameClass :type Save%20Game%20Class%20Reference))
  (bind _returnvalue (SaveGame|DoesSaveGameExist SlotName UserIndex))
  (if _returnvalue
    (bind _returnvalue_2 (SaveGame|LoadGamefromSlot SlotName UserIndex))
    (bind _asgame_save (Utilities|Casting|CastToGameSave _returnvalue_2))
    (Variables|SaveActor|SetGameSave _asgame_save)
    (Variables|Default|SetLoadedFromSaveGame? true)
    (else
      (bind _returnvalue_3 (SaveGame|CreateSaveGameObject SaveGameClass))
      (bind _asgame_save_2 (Utilities|Casting|CastToGameSave _returnvalue_3))
      (Variables|SaveActor|SetGameSave _asgame_save_2)
      (Variables|Default|SetLoadedFromSaveGame? false)))
  (return (Variables|SaveActor|GetGameSave) (Variables|Default|GetLoadedFromSaveGame?)))

(fn LoadSaveableObjectsIntoArray
  (params (Current%20Iterator :type Integer))
  (bind _index (Utilities|FlowControl|ForLoopwithBreak Current%20Iterator (Utilities|Array|LastIndex (Variables|Default|GetCached%20SavableObjects)))
    (:LoopBody
      (LocalVariables|SetCurrentIndex _index)
      (Class|SaveAbleBp|GetSavableValues(Message) (Utilities|Array|Get(acopy) (Variables|Default|GetCached%20SavableObjects) (LocalVariables|GetCurrentIndex)))
      (Variables|Default|SetCurrentloopCounter 0))))