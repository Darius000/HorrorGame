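; Checkpoint actor that notifies the SaveManager the first time a ThirdPersonCharacter overlaps it.
; The overlap calls CheckPoint on a valid SaveManager and sets CheckPointReached, which blocks later triggers.
; GetSaveableValues packs that flag and a self reference into a saveable struct with a newly generated GUID on every call, while DidInteractWith? sets the flag from its input.
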(event Collision|EventActorBeginOverlap
  (params (OtherActor :type Actor%20Object%20Reference))
  (bind _savemanager (Variables|Default|GetSaveManager))
  (Utilities|Casting|CastToThirdPersonCharacter OtherActor)
  (if (not (Variables|Default|GetCheckPointReached))
    (if (!= _savemanager 0)
      (Default|CheckPoint _savemanager self)
      (Variables|Default|SetCheckPointReached true))))

(event EventDidInteractWith?
  (params (InteractedWith :type Boolean))
  (Variables|Default|SetCheckPointReached InteractedWith))

(fn ConstructionScript)

(fn GetSaveableValues
  (return (Utilities|Struct|MakeSTRUCT_SaveableObject (Guid|NewGuid) self (Variables|Default|GetCheckPointReached))))